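; VR push-button mesh component that BP_MotionController presses physically by overlapping it.
; On overlap it enables tick and follows the controller's GrabSphere along local Z, clamped to a maximum travel.
; When the controller leaves, it interpolates back at constant speed, disabling tick once its return check passes.
; Crossing the activation depth flips its state and green/red material, calling CallButtonPressed subject to a minimum interval.
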(event Custom|ComponentBeginOverlap
  (params (OverlappedComponent :type Primitive%20Component%20Object%20Reference) (OtherActor :type Actor%20Object%20Reference) (OtherComp :type Primitive%20Component%20Object%20Reference) (OtherBodyIndex :type Integer) (bFromSweep :type Boolean) (SweepResult :type Hit%20Result%20Structure%20%28by%20ref%29))
  ;[1 0.007073 0] Events
  ;[1 0.7652 0] То, на что кнопка будет реагировать
  (bind _asbp_motion_controller (Utilities|Casting|CastToBP_MotionController OtherActor)) ; Проверка на коллизию с контроллером
  (Variables|Default|SetFocusedController _asbp_motion_controller)
  (CallFunction|StartButtonTranforming) ; Запуск тика+инициализация трансформов
)

(event Custom|ComponentEndOverlap
  (params (OverlappedComponent :type Primitive%20Component%20Object%20Reference) (OtherActor :type Actor%20Object%20Reference) (OtherComp :type Primitive%20Component%20Object%20Reference) (OtherBodyIndex :type Integer))
  ;[1 0.007073 0] Events
  ;[1 1 1] Отключение кнопки
  (if (Variables|States|GetisEnabled)
    (if (== OtherActor (Variables|Default|GetFocusedController))
      (Variables|States|SetisEnabled false))))

(event EventBeginPlay
  ;[1 0.007073 0] BeginPlay
  ;[1 1 1] Бинд евентов на пересечение с мешем кнопки
  (Collision|BindEventtoOnComponentBeginOverlap (EventDispatchers|CreateEvent :!event Custom|ComponentBeginOverlap))
  (Collision|BindEventtoOnComponentEndOverlap (EventDispatchers|CreateEvent :!event Custom|ComponentEndOverlap))
  ;[1 1 1] Запись начального трансформа кнопки
  (Variables|Transform|SetStartupTransform (Transformation|GetRelativeTransform)))

(event EventTick
  (params (DeltaSeconds :type Float%20%28single-precision%29))
  ;[1 0.02329 0] Tick
  (Utilities|FlowControl|Sequence
    (:then_0
      (if (Variables|States|GetisEnabled)
        (CallFunction|UpdateButtonLocation) ; Обновляем позицию кнопки от контроллера
        (else
          ;[1 1 1] Возврат кнопки в исходное состояние
          (if (not (Variables|States|GetLerping))
            (Variables|Default|SetFocusedController 0)
            (Variables|States|SetLerping true)))))
    (:then_1
      (CallFunction|LerpReturnMovingButton) ; Возврат в исходное состояние
      (CallFunction|UpdateButtonStateandColor) ; Апдейт статуса кнопки и цвета
    )))

(fn GetCurrentTransform
  (Variables|Default|GetFocusedController ; Актор, взаимодействующий\nс кнопкой
    (:then
      ;[1 1 1] Получение относительного трамсформа кнопки от её родителя
      (return (Math|Transform|ComposeTransforms (Variables|Transform|GetStartupTransform) (Transformation|GetWorldTransform (Transformation|GetAttachParent)))))
    (:else
      (return (Variables|Transform|GetStartupTransform)) ; Возврат кнопки на место, если убрать руку
    )))

(fn StartButtonTranforming
  (bind _currenttransform (CallFunction|GetCurrentTransform))
  (Variables|Transform|SetStartupLocalZ (.z (Math|Transform|InverseTransformLocation _currenttransform (Transformation|GetWorldLocation (Variables|/Game/VirtualRealityBP/Blueprints/BP_MotionController.BP_MotionController_C|GetGrabSphere (Variables|Default|GetFocusedController)))))) ; Z контроллера в координатах кнопки
  (Variables|Transform|SetStartupComponentZ (.z (Math|Transform|InverseTransformLocation _currenttransform (Transformation|GetWorldLocation)))) ; Z кнопки
  (Components|Tick|SetComponentTickEnabled true) ; Включаем тик
  ;[1 1 1] Задаем стартовые переменные
  (Variables|States|SetLerping false)
  (Variables|States|SetToggledThisTouch false)
  (Variables|States|SetisEnabled true))

(fn CheckButtonPressed
  (params (State :type Boolean))
  (if (>= (Math|Timespan|GetTotalSeconds (- (Math|DateTime|Now) (Variables|Default|GetLastToggleTime))) (Variables|MainSettings|GetMinTimeBetweenToggle)) ; Прошло ли время с последнего нажатия?
    (bind _output_get (Variables|States|SetButtonState State))
    (Default|CallButtonPressed _output_get) ; Вызов нажатия и отжатия кнопки
    (Variables|Default|SetLastToggleTime (Math|DateTime|Now))
    (else
      (return false))))

(fn SetButtonColor
  (if (Variables|States|GetButtonState)
    (Rendering|Material|SetMaterial 0 "/Game/Materials/MI_GreenColor.MI_GreenColor")
    (else
      (Rendering|Material|SetMaterial 0 "/Game/Materials/MI_RedColor.MI_RedColor"))))

(fn UpdateButtonLocation
  (bind _currenttransform (CallFunction|GetCurrentTransform))
  (bind _maxmovedistance (Variables|MainSettings|GetMaxMoveDistance))
  (bind _focusedcontroller (Variables|Default|GetFocusedController))
  (bind _startuplocalz (Variables|Transform|GetStartupLocalZ))
  (bind _grabsphere (Variables|/Game/VirtualRealityBP/Blueprints/BP_MotionController.BP_MotionController_C|GetGrabSphere _focusedcontroller))
  (bind _returnvalue (Transformation|GetWorldLocation _grabsphere))
  (bind _returnvalue_2 (Math|Transform|InverseTransformLocation _currenttransform _returnvalue))
  (bind _returnvalue_3 (- _startuplocalz (.z _returnvalue_2)))
  (bind _returnvalue_4 (Math|Float|Clamp(Float) _returnvalue_3 0.0 _maxmovedistance))
  (if (> _returnvalue_4 0.0) ; Текущий трансофрм кнопки отличен от нуля?
    (Transformation|SetRelativeLocation (Math|Transform|TransformLocation (Variables|Transform|GetStartupTransform) (Math|Vector|MakeVector 0.0 0.0 (Math|Float|Clamp(Float) (+ (Variables|Transform|GetStartupComponentZ) (* _returnvalue_4 -1.0)) (* (Variables|MainSettings|GetMaxMoveDistance) -1.0)))) false false)))

(fn LerpReturnMovingButton
  (bind _returnvalue (Utilities|Time|GetWorldDeltaSeconds))
  (bind _startuptransform (Variables|Transform|GetStartupTransform))
  (bind _relativelocation (Variables|Default|GetRelativeLocation))
  (bind _returnspeed (Variables|MainSettings|GetReturnSpeed))
  (bind _returnvalue_2 (Math|Interpolation|VInterptoConstant _relativelocation (.location _startuptransform) _returnvalue _returnspeed))
  (if (Variables|States|GetLerping)
    (Transformation|SetRelativeLocation _returnvalue_2 false false)
    (if (Math|Vector|Equal(Vector) _returnvalue_2 "0, 0, 0" 0.0001) ; Кнопка встала на место?
      (Variables|States|SetLerping false)
      (Components|Tick|SetComponentTickEnabled false))))

(fn UpdateButtonStateandColor
  (bind _togglingzoneheight (Variables|MainSettings|GetTogglingZoneHeight))
  (bind _relativelocation (Variables|Default|GetRelativeLocation))
  (bind _startuptransform (Variables|Transform|GetStartupTransform))
  (bind _returnvalue (Math|Transform|InverseTransformLocation _startuptransform _relativelocation))
  (bind _returnvalue_2 (* _togglingzoneheight -1.0))
  (bind _returnvalue_3 (+ _returnvalue_2 0.001))
  (bind _returnvalue_4 (<= (.z _returnvalue) _returnvalue_3))
  (if (Math|Boolean|NotEqual(Boolean) _returnvalue_4 (Variables|States|GetButtonState)) ; Кнопка в зоне активации, и ее можно переключить?
    (bind _output_get (Variables|States|SetButtonState _returnvalue_4))
    (CallFunction|CheckButtonPressed _output_get)
    (CallFunction|SetButtonColor)))