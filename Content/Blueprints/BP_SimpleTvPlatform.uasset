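; Interactive TV platform that animates a column's height when interacted with, then starts video playback on the TV.
; TryInteract, an interface event, plays a timeline that drives the column's relative Z.
; On finish, it applies the media material, opens the video source and binds the On/Off button components.
; Off only swaps the screen to a color material without stopping the player; On restores the video material and reopens the source.
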(event Custom|ButtonOffPressed
  (params (ButtonState :type Boolean))
  ;[0.1461 0.151 0.1495] Turn Off event
  (Rendering|Material|SetMaterial (Variables|Default|GetTV) 0 "/Game/Materials/M_Color.M_Color"))

(event Custom|ButtonOnPressed
  (params (ButtonState :type Boolean))
  ;[0.7391 1 0.4582] Turn On event
  (Rendering|Material|SetMaterial (Variables|Default|GetTV) 0 "/Game/Media/SimpleMediaPlayer_Video_Mat.SimpleMediaPlayer_Video_Mat")
  (Media|MediaPlayer|OpenSource (Variables|Default|GetMediaPlayer) "/Game/Media/SimpleVideoFileMediaSource.SimpleVideoFileMediaSource"))

(event EventTryInteract
  (bind _column (Variables|Default|GetColumn))
  (bind _relativelocation (Variables|/Script/Engine.SceneComponent|GetRelativeLocation _column))
  ;[1 0.06264 0] Interact By Interface
  ;[1 1 1] Простая анимация подъема
  (bind _relativelocation_2 (Timeline|PlatforMoving PlayFromStart)
    (:Update
      (Transformation|SetRelativeLocation _column (Math|Vector|MakeVector (.x _relativelocation) (.y _relativelocation) _relativelocation_2) false false))
    (:Finished
      ;[1 1 1] Сетап материала
      (Rendering|Material|SetMaterial (Variables|Default|GetTV) 0 "/Game/Media/SimpleMediaPlayer_Video_Mat.SimpleMediaPlayer_Video_Mat")
      (Media|MediaPlayer|OpenSource (Variables|Default|GetMediaPlayer) "/Game/Media/SimpleVideoFileMediaSource.SimpleVideoFileMediaSource")
      ;[1 1 1] Бинд и кнопок включения и выключения ТВ
      (EventDispatchers|BindEventtoButtonPressed (Variables|Default|GetBPC_ButtonOff) (delegate Custom|ButtonOffPressed))
      (EventDispatchers|BindEventtoButtonPressed (Variables|Default|GetBPC_ButtonOn) (delegate Custom|ButtonOnPressed)))))

(fn ConstructionScript)