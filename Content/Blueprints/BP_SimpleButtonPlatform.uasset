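; BP_SimpleButtonPlatform is a button-mash platform that triggers a linked InteractableActor once its circular progress bar is full.
; BeginPlay binds the button component's press event, overrides the bar's decrease speed, then plays it from empty.
; While the timer is active, each press adds ButtonPower to the current time.
; A press that finds the bar already full stops the timer and sends the interact interface message.
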(event Custom|ButtonPressed
  (params (ButtonState :type Boolean))
  ;[1 0.02878 0] Button Pressed
  (if (and ButtonState (Variables|/Game/Blueprints/BPI_CircleProgressbar.BPI_CircleProgressbar_C|GetisTimerActive (Variables|Default|GetBPI_CircleProgressbar))) ; Кнопка нажата?\nтаймер работает?
    (bind _success (CallFunction|CheckComplete)) ; Проверка на заполнение прогрессбара
    (CallFunction|AddTime (not _success)) ; Добавляем таймеру время от кнопки
    (if _success ; Прогрессбар заполнился?
      ;[1 0.8211 0] Complete Progressbar
      (Default|ForceStopatTime (Variables|Default|GetBPI_CircleProgressbar) 1.0) ; Стоп таймер
      (bind _interactableactor (Variables|Default|GetInteractableActor) ; InteractableActor
        (:then
          (Class|BPIInteract|TryInteract(Message) _interactableactor) ; Взаимодействие через интерфейс
        )
        (:else)))))

(event EventBeginPlay
  (bind _bpi_circleprogressbar (Variables|Default|GetBPI_CircleProgressbar))
  ;[1 0.02878 0] BeginPlay
  ;[1 1 1] Первоначальная настройка кнопки и прогрессбара
  (EventDispatchers|BindEventtoButtonPressed (Variables|Default|GetBPC_Button) (EventDispatchers|CreateEvent :!event Custom|ButtonPressed)) ; Бинд Евента на нажатие кнопки
  (Variables|/Game/Blueprints/BPI_CircleProgressbar.BPI_CircleProgressbar_C|SetDecraseSpeed _bpi_circleprogressbar (Variables|Default|GetDecreaseSpeed)) ; Override скорости убавления прогрессбара
  (Variables|/Game/Blueprints/BPI_CircleProgressbar.BPI_CircleProgressbar_C|SetCurrentTime _bpi_circleprogressbar 0.0)
  (Default|Play _bpi_circleprogressbar))

(fn ConstructionScript)

(fn AddTime
  (params (Condition :type Boolean))
  (if Condition
    (if (<= (Variables|/Game/Blueprints/BPI_CircleProgressbar.BPI_CircleProgressbar_C|GetCurrentTime (Variables|Default|GetBPI_CircleProgressbar)) 1.0)
      (Variables|/Game/Blueprints/BPI_CircleProgressbar.BPI_CircleProgressbar_C|SetCurrentTime (Variables|Default|GetBPI_CircleProgressbar) (+ (Variables|Default|GetButtonPower) (Variables|/Game/Blueprints/BPI_CircleProgressbar.BPI_CircleProgressbar_C|GetCurrentTime (Variables|Default|GetBPI_CircleProgressbar)))))))

(fn CheckComplete
  (if (>= (Variables|/Game/Blueprints/BPI_CircleProgressbar.BPI_CircleProgressbar_C|GetCurrentTime (Variables|Default|GetBPI_CircleProgressbar)) 1.0)
    (return true)
    (else
      (return false))))